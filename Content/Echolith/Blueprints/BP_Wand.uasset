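; Grabbable VR wand that casts the currently selected spell from the holding hand.
; Grabbing enables input, adds that hand's weapon mapping context and hides the hand through a message to the controller's owner, avoiding a hard pawn reference; dropping reverses this.
; The matching shoot input spawns the current spell actor, calls its CastSpell and starts a cooldown timer.
; SetSpellFromEnum picks the spell class from a type-to-class map.
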(event OnGrabbed(GrabComponent)
  (bind _grabcomponent (Variables|Default|GetGrabComponent))
  (bind _returnvalue (Default|GetHeldbyHand _grabcomponent))
  (bind _returnvalue_2 (Utilities|Enum|Equal(Enum) _returnvalue "Right"))
  (Input|EnableInput (Game|GetPlayerController 0))
  (Class|BPIPawnAnim|HideUnhideHand(Message) (Components|GetOwner (Variables|/Game/VRTemplate/Blueprints/GrabComponent.GrabComponent_C|GetMotionControllerRef _grabcomponent)) true _returnvalue_2)
  (Input|AddMappingContext (PlayerController|LocalPlayerSubsystems|GetEnhancedInputLocalPlayerSubsystem (Game|GetPlayerController 0)) (select _returnvalue_2 "/Game/VRTemplate/Input/IMC_Weapon_Right.IMC_Weapon_Right" "/Game/VRTemplate/Input/IMC_Weapon_Left.IMC_Weapon_Left") 1 "(bIgnoreAllPressedKeysUntilRelease=True,bForceImmediately=False,bNotifyUserSettings=False)"))

(event OnDropped(GrabComponent)
  (bind _grabcomponent (Variables|Default|GetGrabComponent))
  (bind _returnvalue (Default|GetHeldbyHand _grabcomponent))
  (bind _returnvalue_2 (Utilities|Enum|Equal(Enum) _returnvalue "Right"))
  (Input|DisableInput (Game|GetPlayerController 0))
  (Class|BPIPawnAnim|HideUnhideHand(Message) (Components|GetOwner (Variables|/Game/VRTemplate/Blueprints/GrabComponent.GrabComponent_C|GetMotionControllerRef _grabcomponent)) false _returnvalue_2)
  (Input|RemoveMappingContext (PlayerController|LocalPlayerSubsystems|GetEnhancedInputLocalPlayerSubsystem (Game|GetPlayerController 0)) (select _returnvalue_2 "/Game/VRTemplate/Input/IMC_Weapon_Right.IMC_Weapon_Right" "/Game/VRTemplate/Input/IMC_Weapon_Left.IMC_Weapon_Left") "(bIgnoreAllPressedKeysUntilRelease=True,bForceImmediately=False,bNotifyUserSettings=False)"))

(event Input|EnhancedActionEvents|EnhancedInputActionIA_Shoot_Left
  (params (ActionValue :type Boolean) (ElapsedSeconds :type Float%20%28double-precision%29) (TriggeredSeconds :type Float%20%28double-precision%29) (InputAction :type Input%20Action%20Object%20Reference :default "/Game/VRTemplate/Input/Actions/IA_Shoot_Left.IA_Shoot_Left"))
  (:Started
    (if (Utilities|Enum|Equal(Enum) (Default|GetHeldbyHand (Variables|Default|GetGrabComponent)) "Left")
      (CallFunction|CastSpell))))

(event Input|EnhancedActionEvents|EnhancedInputActionIA_Shoot_Right
  (params (ActionValue :type Boolean) (ElapsedSeconds :type Float%20%28double-precision%29) (TriggeredSeconds :type Float%20%28double-precision%29) (InputAction :type Input%20Action%20Object%20Reference :default "/Game/VRTemplate/Input/Actions/IA_Shoot_Right.IA_Shoot_Right"))
  (:Started
    (if (Utilities|Enum|Equal(Enum) (Default|GetHeldbyHand (Variables|Default|GetGrabComponent)) "Right")
      (CallFunction|CastSpell))))

(event EventBeginPlay)

(event Collision|EventActorBeginOverlap
  (params (OtherActor :type Actor%20Object%20Reference)))

(event EventTick
  (params (DeltaSeconds :type Float%20%28single-precision%29)))

(fn ConstructionScript)

(fn CastSpell
  (if (Variables|Default|GetbCanCast)
    (Variables|Default|SetbCanCast false)
    (bind _returnvalue (Game|SpawnActorfromClass (Variables|Default|GetCurrentSpellClass) (Math|Conversions|ToTransform(Vector) (Math|Vector|GetForwardVector (Variables|Default|GetSpellSpawnPoint))) "Undefined" "MultiplyWithRoot" 0 (Game|GetInstigator)))
    (Default|CastSpell _returnvalue)
    (Utilities|Time|SetTimerbyFunctionName 0 "ResetCanCast" (Variables|Default|GetSpellCooldown))))

(fn ResetCanCast
  (Variables|Default|SetbCanCast true))

(fn SetSpellfromEnum
  (params (SelectedSpellType :type E_SpellType%20Enum :default "NewEnumerator0"))
  (Variables|Default|SetCurrentSpellClass (.Value (Utilities|Map|Find (Variables|Default|GetSpellTypeToClassMap) SelectedSpellType))))