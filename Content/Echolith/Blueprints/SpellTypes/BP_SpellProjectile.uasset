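; BP_SpellProjectile is a projectile spell that damages the actor it hits.
; CastSpell runs the parent cast, prints a debug message, and passes the mesh's forward vector at a fixed speed to the projectile movement as local-space velocity.
; A mesh hit on a valid actor applies damage credited to the instigator's controller, then destroys the projectile.
; Impact effect and sound nodes exist but never run.
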(event OnComponentHit(StaticMesh)
  (params (HitComponent :type Primitive%20Component%20Object%20Reference) (OtherActor :type Actor%20Object%20Reference) (OtherComp :type Primitive%20Component%20Object%20Reference) (NormalImpulse :type Vector :default "0, 0, 0") (Hit :type Hit%20Result%20Structure%20%28by%20ref%29))
  (if (Utilities|IsValid OtherActor)
    (Game|Damage|ApplyDamage OtherActor (Variables|Default|GetDamage) (Game|GetInstigatorController) self)
    (Actor|DestroyActor)))

(fn ConstructionScript
  (|CallParentFunction))

(fn CastSpell
  (|CallParentFunction)
  (Development|PrintText "--------------------------------------------------------------------------------Projectile Spell Cast")
  (Game|Components|ProjectileMovement|SetVelocityinLocalSpace (Variables|Default|GetProjectileMovement) (* (Math|Vector|GetForwardVector (Variables|Default|GetStaticMesh)) 5e+02)))